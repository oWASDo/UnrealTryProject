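; CarController is a test controller that drives a physics-based pawn from the Forward and Right input axes.
; Forward applies a mass-independent force along the forward vector of the pawn's static mesh, scaled by the axis value, and prints that value.
; Right adds a yaw angular impulse as a velocity change to the same mesh, which is looked up from the controlled pawn on each input.
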(event `InputAxis|Forward` :consume false
  (params (AxisValue :type "Float (single-precision)"))
  (bind _returnvalue (`self.GetComponentByClass` (`self.K2_GetPawn`) "/Script/Engine.StaticMeshComponent"))
  (`KismetSystemLibrary.PrintString` (`KismetStringLibrary.Conv_DoubleToString` AxisValue))
  (`PrimitiveComponent.AddForce` _returnvalue (* (* (`SceneComponent.GetForwardVector` _returnvalue) 2000.0) AxisValue) "None" true))

(event `InputAxis|Right` :consume false
  (params (AxisValue :type "Float (single-precision)"))
  (`PrimitiveComponent.AddAngularImpulseInDegrees` (`self.GetComponentByClass` (`self.K2_GetPawn`) "/Script/Engine.StaticMeshComponent") (* (0.0 0.0 30.0) AxisValue) "None" true))

(fn `UserConstructionScript`)