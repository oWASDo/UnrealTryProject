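; Test robot target that shows a floating damage number when a soldier attacks it.
; Attacked spawns a Text actor at the static mesh's transform, displaying a rounded-down random value between the given minimum and maximum damage.
; Both Attacked and Tick run a shared check that resets the Soldier passed to Attacked whenever its animation Blueprint's Damage flag is false.
; No health is tracked or reduced here.
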(event `Attacked`
  (params (MinDamage :type "Float (double-precision)") (MaxDamage :type "Float (double-precision)") (Soldier :type "/Game/Tests/Animation/Soldier Object Reference"))
  (bind _returnvalue (`|SpawnActorFromClass` "/Game/Tests/Blueprint/Strategic/Text.Text_C" (`SceneComponent.K2_GetComponentToWorld` (`self.StaticMeshComponent`)) "AlwaysSpawn" "OverrideRootScale" null null))
  (bind _astext (cast `/Game/Tests/Blueprint/Strategic/Text` _returnvalue))
  (`TextRenderComponent.K2_SetText` (`/Game/Tests/Blueprint/Strategic/Text.TextRender` _astext) (`KismetTextLibrary.Conv_DoubleToText` (`KismetMathLibrary.Conv_IntToDouble` (`KismetMathLibrary.FFloor` (`KismetMathLibrary.RandomFloatInRange` MinDamage MaxDamage))) "HalfToEven"))
  (if (not (`/Game/Tests/Animation/SoldierAnimBP.Damage` (`/Game/Tests/Animation/Soldier.GetAnimationBluprint` Soldier))) :!label _label
    (`/Game/Tests/Animation/Soldier.Reset` Soldier)))

(event `self.ReceiveTick`
  (params (DeltaSeconds :type "Float (single-precision)"))
  (goto _label))

(fn `UserConstructionScript`)