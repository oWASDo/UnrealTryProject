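; Player controller for an RTS-style test, handling camera movement, soldier selection and move orders.
; Axis inputs slide the controlled pawn along its forward and right vectors with sweep, and zoom by adjusting its spring arm length within clamped limits.
; Left click clears the selection, then selects the Soldier under the cursor and shows its Cone marker.
; Right click sends selected soldiers to the cursor's hit location through GoToPoint.
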(event `InputAxis|Forward` :consume false
  (params (AxisValue :type "Float (single-precision)"))
  (`self.MoveTo` AxisValue (`self.Speed`) true))

(event `InputAxis|Right` :consume false
  (params (AxisValue :type "Float (single-precision)"))
  (`self.MoveTo` AxisValue (`self.Speed`)))

(event `InputAxis|Zoom` :consume false
  (params (AxisValue :type "Float (single-precision)"))
  (`self.Zoomming` AxisValue))

(event `InputAction|LeftClick` :consume false
  (params (Key :type "Key Structure"))
  (:`Pressed`
    (`self.Hide`)
    (`self.AddSoldier`)))

(event `InputAction|RIghtClick` :consume false
  (params (Key :type "Key Structure"))
  (:`Pressed`
    (`self.ActivePathFinding`)))

(fn `ActivePathFinding`
  (for _array_element (`self.Soldirs`)
    (`/Game/Tests/Animation/Soldier.GoToPoint` (cast `/Game/Tests/Animation/Soldier` _array_element :!pure true) (`.Location` (`GameplayStatics.BreakHitResult` (`self.GetHitResultUnderCursorByChannel` "TraceTypeQuery2" false))))))

(fn `AddSoldier`
  (bind (_hitresult _returnvalue) (`self.GetHitResultUnderCursorByChannel` "TraceTypeQuery2" false))
  (if _returnvalue
    (bind _assoldier (cast `/Game/Tests/Animation/Soldier` (`.HitActor` (`GameplayStatics.BreakHitResult` _hitresult))))
    (`KismetArrayLibrary.Array_Add` (`self.Soldirs`) _assoldier)
    (`SceneComponent.SetVisibility` (`/Game/Tests/Animation/Soldier.Cone` _assoldier) true true)))

(fn `Hide`
  (bind _soldirs (`self.Soldirs`))
  (for _array_element _soldirs
    (bind _assoldier (cast `/Game/Tests/Animation/Soldier` _array_element))
    (`SceneComponent.SetVisibility` (`/Game/Tests/Animation/Soldier.Cone` _assoldier) false false))
  (`KismetArrayLibrary.Array_Clear` _soldirs))

(fn `MoveTo`
  (params (AccellerationValue :type "Float (double-precision)") (Speed :type "Float (double-precision)") (Forward :type Boolean))
  (bind _returnvalue (`self.K2_GetPawn`))
  (bind _returnvalue_2 (`self.K2_GetPawn`))
  (if Forward
    (set `self.Direction` (`self.GetActorForwardVector` _returnvalue_2))
    (else
      (set `self.Direction` (`self.GetActorRightVector` _returnvalue_2))))
  (`self.K2_SetActorLocation` _returnvalue (+ (`self.K2_GetActorLocation` _returnvalue) (* (`self.Direction`) (* (`GameplayStatics.GetWorldDeltaSeconds`) AccellerationValue Speed))) true false))

(fn `UserConstructionScript`)

(fn `Zoomming`
  (params (AxisValue :type "Float (double-precision)"))
  (bind _asspring_arm_component (cast `SpringArmComponent` (`self.GetComponentByClass` (`self.K2_GetPawn`) "/Script/Engine.SpringArmComponent") :!pure true))
  (set `SpringArmComponent.TargetArmLength` (`KismetMathLibrary.FClamp` (+ (* (`self.ZoomSpeed`) AxisValue) (`SpringArmComponent.TargetArmLength` _asspring_arm_component)) 200.0 1000.0) _asspring_arm_component))