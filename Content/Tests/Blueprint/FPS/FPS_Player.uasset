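; FPS_Player is a test first-person player that locks onto any actor it overlaps and tracks its gun's muzzle position.
; On overlap it prints the actor's name, clears the Move flag on FPS_Controller and snaps to that actor's location and rotation at unit scale.
; The transform lerp uses a full alpha, so the snap is instant and unswept.
; Each tick it stores the world location of the StpidGun Muzzle socket in MuzzlePosition.
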(event `self.ReceiveBeginPlay`)

(event `self.ReceiveActorBeginOverlap`
  (params (OtherActor :type "Actor Object Reference"))
  (`KismetSystemLibrary.PrintString` (`KismetSystemLibrary.GetDisplayName` OtherActor))
  (bind _asfps_controller (cast `/Game/Tests/Blueprint/FPS/FPS_Controller` (`GameplayStatics.GetPlayerController` 0)))
  (set `/Game/Tests/Blueprint/FPS/FPS_Controller.Move?` false _asfps_controller)
  (`self.K2_SetActorTransform` (`KismetMathLibrary.TLerp` (`self.GetTransform`) (`KismetMathLibrary.MakeTransform` (`self.K2_GetActorLocation` OtherActor) (`self.K2_GetActorRotation` OtherActor)) 1.0)))

(event `self.ReceiveTick`
  (params (DeltaSeconds :type "Float (single-precision)"))
  (bind _returnvalue_location (`KismetMathLibrary.BreakTransform` (`SceneComponent.GetSocketTransform` (`self.StpidGun`) "Muzzle" "RTS_World")))
  (set `self.MuzzlePosition` _returnvalue_location))

(fn `UserConstructionScript`)