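; Barrel is a target actor in an FPS Blueprint test that awards a point the first time it registers a hit.
; On Hit, it finds every PointCounter actor in the level and increments its Point.
; The same loop sets the Hitted flag to block repeat scoring and swaps the mesh material to steel, so both changes require a PointCounter to exist.
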(event `self.ReceiveActorBeginOverlap`
  (params (OtherActor :type "Actor Object Reference")))

(event `self.ReceiveTick`
  (params (DeltaSeconds :type "Float (single-precision)")))

(event `self.ReceiveHit`
  (params (MyComp :type "PrimitiveComponent Object Reference") (Other :type "Actor Object Reference") (OtherComp :type "PrimitiveComponent Object Reference") (bSelfMoved :type Boolean) (HitLocation :type "Vector Structure") (HitNormal :type "Vector Structure") (NormalImpulse :type "Vector Structure") (Hit :type "HitResult Structure (by ref)"))
  (if (not (`self.Hitted`))
    (bind _outactors (`GameplayStatics.GetAllActorsOfClass` "/Game/Tests/Blueprint/Strategic/PointCounter.PointCounter_C"))
    (for _array_element _outactors
      (bind _aspoint_counter (cast `/Game/Tests/Blueprint/Strategic/PointCounter` _array_element))
      (set `/Game/Tests/Blueprint/Strategic/PointCounter.Point` (+ (`/Game/Tests/Blueprint/Strategic/PointCounter.Point` _aspoint_counter) 1) _aspoint_counter)
      (set `self.Hitted` true)
      (`PrimitiveComponent.SetMaterial` (`self.StaticMesh`) 0 "/Game/StarterContent/Materials/M_Metal_Steel.M_Metal_Steel"))))

(fn `UserConstructionScript`)