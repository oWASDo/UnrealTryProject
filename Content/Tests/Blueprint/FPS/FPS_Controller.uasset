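; First-person shooter controller that handles movement, mouse look and firing for the controlled pawn.
; Forward and Right axes move the pawn horizontally without sweep via MoveTo, scaled by speed and delta time, while Move is true.
; Both mouse axes share one root-rotation update, with pitch clamped by Control.
; Fire spawns a projectile and sound at the FPS_Player muzzle only while Move is false; E sets Move true.
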(event `InputAxis|Forward` :consume false
  (params (AxisValue :type "Float (single-precision)"))
  (bind _returnvalue (`self.K2_GetPawn`))
  (bind (_returnvalue_x _returnvalue_y) (`KismetMathLibrary.BreakVector` (`self.GetActorForwardVector` _returnvalue)))
  ;[1 1 1] Forward Move
  (if (`self.Move?`)
    (`self.MoveTo` _returnvalue AxisValue (`self.Speed`) (`GameplayStatics.GetWorldDeltaSeconds`) (`KismetMathLibrary.MakeVector` _returnvalue_x _returnvalue_y))))

(event `InputAxis|Right` :consume false
  (params (AxisValue :type "Float (single-precision)"))
  (bind _returnvalue (`self.K2_GetPawn`))
  (bind (_returnvalue_x _returnvalue_y) (`KismetMathLibrary.BreakVector` (`self.GetActorRightVector` _returnvalue)))
  ;[1 1 1] Right Move
  (if (`self.Move?`)
    (`self.MoveTo` _returnvalue AxisValue (`self.Speed`) (`GameplayStatics.GetWorldDeltaSeconds`) (`KismetMathLibrary.MakeVector` _returnvalue_x _returnvalue_y))))

(event `InputAxis|MouseAxisY`
  (params (AxisValue :type "Float (single-precision)"))
  (bind _rootcomponent (`Actor.RootComponent` (`self.K2_GetPawn`)))
  (bind (_returnvalue_roll _returnvalue_pitch _returnvalue_yaw) (`KismetMathLibrary.BreakRotator` (`SceneComponent.K2_GetComponentRotation` _rootcomponent)))
  ;[1 1 1] Mouse Moviment
  (bind _output_get (set `self.Rot` (`KismetMathLibrary.MakeRotator` 0.0 (+ _returnvalue_pitch AxisValue) (+ (stale `InputAxis|MouseAxisX` AxisValue) _returnvalue_yaw)) :!label _label))
  (bind _outfloat (`self.Control` (.pitch _output_get)))
  (`SceneComponent.K2_SetWorldRotation` _rootcomponent (`KismetMathLibrary.MakeRotator` (.roll _output_get) _outfloat (.yaw _output_get)) false false))

(event `InputAxis|MouseAxisX` :consume false
  (params (AxisValue :type "Float (single-precision)"))
  ;[1 1 1] Mouse Moviment
  (goto _label))

(event `InputAction|Fire`
  (params (Key :type "Key Structure"))
  (bind _returnvalue (`self.K2_GetPawn`))
  ;[1 1 1] Shoot
  (:`Pressed`
    (if (not (`self.Move?`))
      (bind _asfps_player (cast `/Game/Tests/Blueprint/FPS/FPS_Player` _returnvalue))
      (bind _muzzleposition (`/Game/Tests/Blueprint/FPS/FPS_Player.MuzzlePosition` _asfps_player))
      (`|SpawnActorFromClass` "/Game/Tests/Blueprint/FPS/ProjectileBp.ProjectileBp_C" (`KismetMathLibrary.MakeTransform` _muzzleposition (`SceneComponent.K2_GetComponentRotation` (`Actor.RootComponent` _returnvalue)) (0.2 0.2 0.2)) "AlwaysSpawn" "OverrideRootScale" null null)
      (`GameplayStatics.PlaySoundAtLocation` "/Game/Tests/Audio/AWP_Shoot_Sound_Effect_CSGO_Cue.AWP_Shoot_Sound_Effect_CSGO_Cue" _muzzleposition))))

(event `Key|E`
  (params (Key :type "Key Structure"))
  (:`Pressed`
    (set `self.Move?` true)))

(fn `Control`
  (params (InFloat :type "Float (double-precision)"))
  (returns (OutFloat :type "Float (double-precision)"))
  (if (> InFloat 85.0)
    (return 85.0)
    (elif (< InFloat -60.0)
      (return -60.0)
      (else
        (return InFloat)))))

(fn `MoveTo`
  (params (PawnTarget :type "Actor Object Reference") (AxisValue :type "Float (double-precision)") (Speed :type "Float (double-precision)") (DeltaTime :type "Float (double-precision)") (Direction :type "Vector Structure"))
  (`self.K2_SetActorLocation` PawnTarget (+ (* Direction (* AxisValue Speed DeltaTime)) (* (`self.K2_GetActorLocation` PawnTarget) 1.0)) false false))

(fn `UserConstructionScript`)